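; BP_Tunnel is an endless-runner tunnel segment with a spinning holed wall, optional health pack and an enemy.
; Crossing TriggerZone asks TunnelSpawner for the next segment, destroys this one, adds score and boosts player speed at score thresholds.
; Overlaps drive BP_Player health, score, health bar and restart on death, while projectiles destroy the enemy for points.
; RandomizeWall and RandomizeHealth vary the wall mesh and roll, and pack presence and position.
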(event `self.ReceiveTick`
  (params (DeltaSeconds :type "Float (single-precision)"))
  (`SceneComponent.K2_AddLocalRotation` (`self.WallMesh`) (`KismetMathLibrary.MakeRotator` (* DeltaSeconds (`self.RotateSpeed`))) false false))

(event `self.TriggerZone.OnComponentBeginOverlap`
  (params (OverlappedComponent :type "PrimitiveComponent Object Reference") (OtherActor :type "Actor Object Reference") (OtherComp :type "PrimitiveComponent Object Reference") (OtherBodyIndex :type Integer) (bFromSweep :type Boolean) (SweepResult :type "HitResult Structure (by ref)"))
  (bind _asbp_player (cast `/Game/InfiniteMatrix/Blueprints/BP_Player` OtherActor))
  (`/Game/InfiniteMatrix/Blueprints/BP_TunnelSpawner.SpawnTunnelAtSpawnPoint` (`self.TunnelSpawner`))
  (`self.K2_DestroyActor`)
  (bind _output_get (set `/Game/InfiniteMatrix/Blueprints/BP_Player.Score` (+ (`/Game/InfiniteMatrix/Blueprints/BP_Player.Score` _asbp_player) 10.0) _asbp_player))
  (if (or (== _output_get 30.0) (== _output_get 70.0) (== _output_get 90.0) (>= _output_get 120.0))
    (set `/Game/InfiniteMatrix/Blueprints/BP_Player.ForwardSpeed` (+ (`/Game/InfiniteMatrix/Blueprints/BP_Player.ForwardSpeed` _asbp_player) 500.0) _asbp_player)))

(event `self.WallMesh.OnComponentBeginOverlap`
  (params (OverlappedComponent :type "PrimitiveComponent Object Reference") (OtherActor :type "Actor Object Reference") (OtherComp :type "PrimitiveComponent Object Reference") (OtherBodyIndex :type Integer) (bFromSweep :type Boolean) (SweepResult :type "HitResult Structure (by ref)"))
  (bind _asbp_player (cast `/Game/InfiniteMatrix/Blueprints/BP_Player` OtherActor))
  (`GameplayStatics.PlayWorldCameraShake` "/Game/InfiniteMatrix/Blueprints/CameraShake.CameraShake_C" (`self.K2_GetActorLocation` (`GameplayStatics.GetPlayerPawn` 0)) 0.0 3000.0)
  (set `/Game/InfiniteMatrix/Blueprints/BP_Player.Score` (- (`/Game/InfiniteMatrix/Blueprints/BP_Player.Score` _asbp_player) 10.0) _asbp_player)
  (if (`/Game/InfiniteMatrix/Blueprints/BP_Player.IsDead` _asbp_player)
    (`/Game/InfiniteMatrix/Blueprints/BP_Player.DisplayRestart` _asbp_player :!label _label)
    (else
      (bind _output_get (set `/Game/InfiniteMatrix/Blueprints/BP_Player.Health` (- (`/Game/InfiniteMatrix/Blueprints/BP_Player.Health` _asbp_player) 10.0) _asbp_player))
      (set `ProgressBar.Percent` (/ _output_get (`/Game/InfiniteMatrix/Blueprints/BP_Player.MaxHealth` _asbp_player)) (`/Game/InfiniteMatrix/Blueprints/HUD.ProgressBar_43` (`/Game/InfiniteMatrix/Blueprints/BP_Player.PROGRESSBAR` _asbp_player)))
      (if (<= _output_get 0.0)
        (set `/Game/InfiniteMatrix/Blueprints/BP_Player.IsDead` true _asbp_player)
        (goto _label)
        (else
          (`/Game/InfiniteMatrix/Blueprints/BP_Player.UpdateHealth` _asbp_player))))))

(event `self.HealthPack.OnComponentBeginOverlap`
  (params (OverlappedComponent :type "PrimitiveComponent Object Reference") (OtherActor :type "Actor Object Reference") (OtherComp :type "PrimitiveComponent Object Reference") (OtherBodyIndex :type Integer) (bFromSweep :type Boolean) (SweepResult :type "HitResult Structure (by ref)"))
  (bind _asbp_player (cast `/Game/InfiniteMatrix/Blueprints/BP_Player` OtherActor))
  (bind _returnvalue (+ (`/Game/InfiniteMatrix/Blueprints/BP_Player.Health` _asbp_player) 10.0))
  (if (<= _returnvalue 100.0)
    (bind _output_get (set `/Game/InfiniteMatrix/Blueprints/BP_Player.Health` _returnvalue _asbp_player))
    (set `ProgressBar.Percent` (/ _output_get 100.0) (`/Game/InfiniteMatrix/Blueprints/HUD.ProgressBar_43` (`/Game/InfiniteMatrix/Blueprints/BP_Player.PROGRESSBAR` _asbp_player)))
    (`ActorComponent.K2_DestroyComponent` (`self.HealthPack`))))

(event `self.Enemy .OnComponentBeginOverlap`
  (params (OverlappedComponent :type "PrimitiveComponent Object Reference") (OtherActor :type "Actor Object Reference") (OtherComp :type "PrimitiveComponent Object Reference") (OtherBodyIndex :type Integer) (bFromSweep :type Boolean) (SweepResult :type "HitResult Structure (by ref)"))
  (bind _playerref (`self.playerref`))
  (bind _asbp_player (cast `/Game/InfiniteMatrix/Blueprints/BP_Player` OtherActor)
    (:`then`
      (bind _output_get (set `/Game/InfiniteMatrix/Blueprints/BP_Player.Health` (+ (`/Game/InfiniteMatrix/Blueprints/BP_Player.Health` _asbp_player) -10.0) _asbp_player))
      (`GameplayStatics.PlayWorldCameraShake` "/Game/InfiniteMatrix/Blueprints/CameraShake.CameraShake_C" (`self.K2_GetActorLocation` (`GameplayStatics.GetPlayerPawn` 0)) 0.0 3000.0)
      (set `ProgressBar.Percent` (/ _output_get 100.0) (`/Game/InfiniteMatrix/Blueprints/HUD.ProgressBar_43` (`/Game/InfiniteMatrix/Blueprints/BP_Player.PROGRESSBAR` _asbp_player)))
      (`ActorComponent.K2_DestroyComponent` (`self.Enemy `))
      (if (<= _output_get 0.0)
        (set `/Game/InfiniteMatrix/Blueprints/BP_Player.IsDead` true _asbp_player)
        (`/Game/InfiniteMatrix/Blueprints/BP_Player.DisplayRestart` _asbp_player)))
    (:`CastFailed`
      (cast `/Game/InfiniteMatrix/Blueprints/BP_Projectile` OtherActor)
      (set `/Game/InfiniteMatrix/Blueprints/BP_Player.Score` (+ (`/Game/InfiniteMatrix/Blueprints/BP_Player.Score` _playerref) 10.0) _playerref)
      (`GameplayStatics.PlaySoundAtLocation` "/Game/InfiniteMatrix/Blueprints/ScoreSound.ScoreSound" (0.0 0.0 0.0) (struct) 1.0 1.0 0.0 null null null null)
      (`ActorComponent.K2_DestroyComponent` (`self.Enemy `)))))

(fn `Randomize Health`
  (bind _healthpack (`self.HealthPack`))
  (if (== (`KismetMathLibrary.RandomIntegerInRange` 0 5) 5)
    (`StaticMeshComponent.SetStaticMesh` _healthpack "/Game/InfiniteMatrix/Meshes/SM_HealthPack.SM_HealthPack")
    (`SceneComponent.K2_SetRelativeLocation` (`self.HealthPack`) (`KismetMathLibrary.MakeVector` (`KismetMathLibrary.RandomFloatInRange` 1000.0 2000.0) (`KismetMathLibrary.RandomFloatInRange` -350.0 350.0) (`KismetMathLibrary.RandomFloatInRange` -350.0 350.0)) false false)
    (else
      (`ActorComponent.K2_DestroyComponent` _healthpack))))

(fn `RandomizeWall`
  (`StaticMeshComponent.SetStaticMesh` (`self.WallMesh`) (select `int` (`KismetMathLibrary.RandomIntegerInRange` 0 3) :`0` "/Game/InfiniteMatrix/Meshes/SM_Hole_01.SM_Hole_01" :`1` "/Game/InfiniteMatrix/Meshes/SM_Hole_02.SM_Hole_02" :`2` "/Game/InfiniteMatrix/Meshes/SM_Hole_03.SM_Hole_03" :`3` "/Game/InfiniteMatrix/Meshes/SM_Hole_04.SM_Hole_04" :!type "StaticMesh Object Reference"))
  (`SceneComponent.K2_AddLocalRotation` (`self.WallMesh`) (`KismetMathLibrary.MakeRotator` (`KismetMathLibrary.RandomFloatInRange` 0.0 360.0)) false false))

(fn `UserConstructionScript`)